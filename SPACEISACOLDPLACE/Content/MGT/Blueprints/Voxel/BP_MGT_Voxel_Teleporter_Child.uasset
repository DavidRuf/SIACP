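; Voxel teleporter child Blueprint that links itself to a gravity generator at runtime.
; On BeginPlay it searches the actors attached to VoxelGravityGenerator and stores the first BP_MGT_GravityGenerator as TargetedGenerator.
; If none is found, it prints a warning and repeats the search after a short delay until the target is valid.
; The construction script only runs the parent's.
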(event `self.ReceiveBeginPlay`
  (for _array_element (`self.GetAttachedActors` (`self.VoxelGravityGenerator`) true) :!label _label
    (bind _asbp_mgt_gravity_generator (cast `/Game/MGT/Blueprints/DynamicGravityGenerators/ParentMatrice/BP_MGT_GravityGenerator` _array_element))
    (set `self.TargetedGenerator` _asbp_mgt_gravity_generator)
    (break))
  (`/Engine/EditorBlueprintResources/StandardMacros.IsValid` (`self.TargetedGenerator`)
    (:`Is Not Valid`
      (`KismetSystemLibrary.PrintString` (`KismetStringLibrary.Concat_StrStr` (`KismetSystemLibrary.GetDisplayName` self) " doesn't find generator") true true (struct :`R` 1.0 :`B` 0.018845 :`A` 1.0))
      (`KismetSystemLibrary.Delay` 1.0)
      (goto _label))))

(fn `UserConstructionScript`
  (`parent.UserConstructionScript`))